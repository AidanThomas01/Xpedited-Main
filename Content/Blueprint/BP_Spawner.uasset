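; BP_Spawner fills the level with Parcel_Box actors when play begins.
; On BeginPlay it sets its child actor's class, then spawns a random number of boxes in a row from Spawner1's location, stepping a running offset along world X.
; Each class comes from a random Select whose two options are both Parcel_Box, though the random range also allows a third, unlisted index.
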(event `self.ReceiveBeginPlay`
  (bind _returnvalue (select `int` (`KismetMathLibrary.RandomIntegerInRange` 0 2) :`0` "/Game/Parcel_Box.Parcel_Box_C" :`1` "/Game/Parcel_Box.Parcel_Box_C" :!type "Actor Class Reference"))
  (`ChildActorComponent.SetChildActorClass` (`self.ChildActor`) _returnvalue)
  (for _ (range (+ (`KismetMathLibrary.RandomInteger` 15) 1))
    (set `self.Spawner1Used` (+ (`self.Spawner1Used`) 100))
    (`|SpawnActorFromClass` _returnvalue (`KismetMathLibrary.Conv_VectorToTransform` (+ (`SceneComponent.K2_GetComponentLocation` (`self.Spawner1`)) (`KismetMathLibrary.MakeVector` (`self.Spawner1Used`)))) "Undefined" "MultiplyWithRoot" null null)))

(fn `UserConstructionScript`)