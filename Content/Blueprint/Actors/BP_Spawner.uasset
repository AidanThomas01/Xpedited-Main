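; BP_Spawner is an actor that fills the level with Parcel_Box packages when play begins.
; It sets its child actor to Parcel_Box, rolls a random package count and reports that count plus three to the first-person character's UI.
; A tick later, it spawns boxes in a row along world X from Spawner1, using a growing offset.
; The random class selects currently resolve only to Parcel_Box.
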(event `self.ReceiveBeginPlay`
  (bind _amountofpackagesspawnt (`self.AmountOfPackagesSpawnt`))
  (bind _returnvalue (select `int` (`KismetMathLibrary.RandomIntegerInRange` 1 1) :`0` "/Game/Assets/Parcels/Parcel_Box.Parcel_Box_C" :`1` "/Game/Assets/Parcels/Parcel_Box.Parcel_Box_C" :!type "Actor Class Reference"))
  (`ChildActorComponent.SetChildActorClass` (`self.ChildActor`) _returnvalue)
  (set `self.AmountOfPackagesSpawnt` (`KismetMathLibrary.RandomIntegerInRange` 4 15))
  (bind _asbp_first_person_character (cast `/Game/FirstPerson/Blueprints/BP_FirstPersonCharacter` (`GameplayStatics.GetPlayerCharacter` 0)))
  (`/Game/UI/WB_UI_GAME1.INFORMATIONPARCELCREATER` (`/Game/FirstPerson/Blueprints/BP_FirstPersonCharacter.UIReference` _asbp_first_person_character) (+ _amountofpackagesspawnt 3))
  (`KismetSystemLibrary.DelayUntilNextTick`)
  (for _ (range (+ _amountofpackagesspawnt 1))
    (set `self.Spawner1Used` (+ (`self.Spawner1Used`) 100))
    (`|SpawnActorFromClass` _returnvalue (`KismetMathLibrary.Conv_VectorToTransform` (+ (`SceneComponent.K2_GetComponentLocation` (`self.Spawner1`)) (`KismetMathLibrary.MakeVector` (`self.Spawner1Used`)))) "Undefined" "MultiplyWithRoot" null null)))

(fn `UserConstructionScript`)